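; BP_engimeBall is an actor that destroys itself when a Bp_BallActor overlaps its static mesh, apparently part of a ball puzzle in a test level.
; The construction script sizes and positions a Box component to match the bounds of the assigned mesh.
; Only the mesh's overlap event carries logic; the hit event is empty and the Box has no events in the graph.
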(event OnComponentHit(StaticMesh)
  (params (HitComponent :type Primitive%20Component%20Object%20Reference) (OtherActor :type Actor%20Object%20Reference) (OtherComp :type Primitive%20Component%20Object%20Reference) (NormalImpulse :type Vector :default "0, 0, 0") (Hit :type Hit%20Result%20Structure%20%28by%20ref%29)))

(event OnComponentBeginOverlap(StaticMesh)
  (params (OverlappedComponent :type Primitive%20Component%20Object%20Reference) (OtherActor :type Actor%20Object%20Reference) (OtherComp :type Primitive%20Component%20Object%20Reference) (OtherBodyIndex :type Integer) (bFromSweep :type Boolean) (SweepResult :type Hit%20Result%20Structure%20%28by%20ref%29))
  (Utilities|Casting|CastToBp_BallActor OtherActor)
  (Actor|DestroyActor))

(event EventBeginPlay)

(event Collision|EventActorBeginOverlap
  (params (OtherActor :type Actor%20Object%20Reference)))

(event EventTick
  (params (DeltaSeconds :type Float%20%28single-precision%29)))

(fn ConstructionScript
  (bind _staticmesh (Variables|Default|GetStaticMesh))
  (bind _box (Variables|Default|GetBox))
  (bind _staticmesh_2 (Variables|/Script/Engine.StaticMeshComponent|GetStaticMesh _staticmesh))
  (bind _returnvalue (StaticMesh|GetBounds _staticmesh_2))
  (Components|Box|SetBoxExtent _box (.boxextent _returnvalue) true)
  (Transformation|SetRelativeLocation _box (.origin _returnvalue) false false))