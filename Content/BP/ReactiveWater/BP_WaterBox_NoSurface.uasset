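; Surfaceless water volume that can send the player back to a Respawn point on contact.
; Construction script sizes the underwater plane from EndPoint and the Box and KillBox from UnderwaterHeight.
; UseUnderwaterPlane toggles plane visibility and post-process weight, but only applies when WaterKill is on.
; With WaterKill, KillBox overlap by the player character spawns fall Niagara effects, blocks game input, then teleports player 0's capsule after a short delay.
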(event OnComponentBeginOverlap(KillBox)
  (params (OverlappedComponent :type Primitive%20Component%20Object%20Reference) (OtherActor :type Actor%20Object%20Reference) (OtherComp :type Primitive%20Component%20Object%20Reference) (OtherBodyIndex :type Integer) (bFromSweep :type Boolean) (SweepResult :type Hit%20Result%20Structure%20%28by%20ref%29))
  (bind _returnvalue (Game|GetPlayerController 0))
  (if (Variables|00-WaterConstruction|GetWater%20Kill?)
    (Utilities|Casting|CastToMyMyProject8Character OtherActor)
    (Niagara|SpawnSystematLocation "/Game/VFX/Waterfall/NS_Waterfall_PlayerFall.NS_Waterfall_PlayerFall" (Transformation|GetWorldLocation (Variables|/Script/Engine.Character|GetCapsuleComponent (Game|GetPlayerCharacter 0))))
    (Input|SetInputModeUIOnly _returnvalue 0 "DoNotLock" true)
    (Utilities|FlowControl|Delay 0.5)
    (Transformation|SetWorldLocation (Variables|/Script/Engine.Character|GetCapsuleComponent (Game|GetPlayerCharacter 0)) (Transformation|GetWorldLocation (Variables|Default|GetRespawn)) false true)
    (Input|SetInputModeGameOnly _returnvalue true)))

(fn ConstructionScript
  (bind _end_point (Variables|00-WaterConstruction|GetEnd%20Point))
  (bind _killbox (Variables|Default|GetKillBox))
  (bind _killbox_2 (Variables|Default|GetKillBox))
  (bind _sm_underwaterplane (Variables|Default|GetSM_UnderwaterPlane))
  (bind _postprocess (Variables|Default|GetPostProcess))
  (bind _returnvalue (/ _end_point 1e+02))
  (Transformation|SetWorldScale3D (Variables|Default|GetSM_UnderwaterPlane) (Math|Vector|MakeVector (.x _returnvalue) (.y _returnvalue) 1.0))
  (Transformation|SetRelativeScale3D (Variables|Default|GetBox) (Math|Vector|MakeVector 1.0 1.0 (Variables|00-WaterConstruction|GetUnderwater%20Height)))
  (Transformation|SetRelativeLocation (Variables|Default|GetBox) (Math|Vector|MakeVector 1.0 1.0 (* (Variables|00-WaterConstruction|GetUnderwater%20Height) -1.0)) false false)
  (Rendering|Material|SetMaterial (Variables|Default|GetSM_UnderwaterPlane) 0 (Variables|00-WaterConstruction|GetUnderwater%20Plane%20Material))
  (if (Variables|00-WaterConstruction|GetWater%20Kill?)
    (Rendering|SetVisibility _killbox_2 true false)
    (Transformation|SetRelativeLocation _killbox (Math|Vector|MakeVector 1.0 1.0 (* (Variables|00-WaterConstruction|GetUnderwater%20Height) (+ (Variables|00-WaterConstruction|GetUnderwater%20Killbox%20Offset) -1.0))) false false)
    (Transformation|SetRelativeScale3D _killbox (Math|Vector|MakeVector 1.0 1.0 (Variables|00-WaterConstruction|GetUnderwater%20Height)))
    (if (Variables|Default|GetUse%20Underwater%20Plane?)
      (Rendering|SetVisibility _sm_underwaterplane true false)
      (Variables|/Script/Engine.PostProcessComponent|SetBlendWeight _postprocess 1.0)
      (else
        (Rendering|SetVisibility _sm_underwaterplane false false)
        (Variables|/Script/Engine.PostProcessComponent|SetBlendWeight _postprocess 0.0)))
    (else
      (Rendering|SetVisibility _killbox_2 false false))))