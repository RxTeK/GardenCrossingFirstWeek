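; BP_WaterComponent makes its owning actor disturb reactive water by applying splats to a BP_WaterSurface.
; Every tick it line traces from the bottom center of the owner's bounds, with a zero offset vector scaled by TraceDistance, against one object type.
; When the hit's PhysMat casts to BP_WaterSurface, it calls ApplyLocalSplat at the owner's location using ImpactSize.
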(event EventTick
  (params (DeltaSeconds :type Float%20%28single-precision%29))
  (bind _returnvalue (Components|GetOwner))
  (bind (_origin _boxextent) (Collision|GetActorBounds _returnvalue false false))
  (bind _returnvalue_2 (- (.z _origin) (.z _boxextent)))
  (bind _returnvalue_3 (Math|Vector|MakeVector (.x _origin) (.y _origin) _returnvalue_2))
  (Utilities|IsValid (Components|GetOwner)
    (:Is%20Valid
      (bind _outhit (Collision|LineTraceForObjects _returnvalue_3 (+ _returnvalue_3 (* "" (Variables|Default|GetTrace%20Distance))) (Utilities|Array|MakeArray "ObjectTypeQuery7") false 0 "None"))
      (bind _output_get (Variables|Default|SetHit _outhit))
      (bind _asbp_water_surface (Utilities|Casting|CastToBP_WaterSurface (.PhysMat (Collision|BreakHitResult _output_get))))
      (bind _output_get_2 (Variables|Default|SetReactive%20Water _asbp_water_surface))
      (Default|ApplyLocalSplat _output_get_2 (Transformation|GetActorLocation (Components|GetOwner)) (Variables|Default|GetImpact%20Size)))))