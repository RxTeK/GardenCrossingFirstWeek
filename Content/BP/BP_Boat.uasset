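; BP_Boat is a boat actor that travels along a spline once the player character enters its trigger box.
; The first overlap starts a looping timer of roughly 60Hz and blends the player's view to the boat.
; MoveBoat increments Speed, which serves as a progress alpha rather than a velocity, to set position and rotation from the referenced BpSPline's length.
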(event OnComponentBeginOverlap(Box)
  (params (OverlappedComponent :type Primitive%20Component%20Object%20Reference) (OtherActor :type Actor%20Object%20Reference) (OtherComp :type Primitive%20Component%20Object%20Reference) (OtherBodyIndex :type Integer) (bFromSweep :type Boolean) (SweepResult :type Hit%20Result%20Structure%20%28by%20ref%29))
  (Utilities|Casting|CastToMyMyProject8Character OtherActor)
  (Utilities|FlowControl|DoOnce false
    (:Completed
      (Utilities|Time|SetTimerbyEvent (EventDispatchers|CreateEvent :!event Custom|MoveBoat) 0.016 true)
      (Game|Player|SetViewTargetwithBlend (Game|GetPlayerController 0) self 1.0 "VTBlend_Linear" 0.0 false))))

(event Custom|MoveBoat
  (bind _bp_spline (Variables|Default|GetBp_SPline))
  (bind _spline (Variables|/Game/BP/BP_SPline.BP_SPline_C|GetSpline _bp_spline))
  (Variables|Default|SetSpeed (+ (Variables|Default|GetSpeed) 0.001))
  (Transformation|SetActorLocationAndRotation (Spline|GetLocationatDistanceAlongSpline _spline (Math|Float|Lerp 0.0 (Spline|GetSplineLength _spline) (+ (Variables|Default|GetSpeed) 0.001)) "World") (Spline|GetRotationatDistanceAlongSpline (Variables|/Game/BP/BP_SPline.BP_SPline_C|GetSpline (Variables|Default|GetBp_SPline)) (Math|Float|Lerp 0.0 (Spline|GetSplineLength _spline) (+ (Variables|Default|GetSpeed) 0.001)) "World")))

(fn ConstructionScript)